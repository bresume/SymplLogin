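; BP_LoginSaveGame is a save game object that stores login details: the remember flag, user name, password and guest status.
; Getter functions expose each stored value.
; SetData writes all fields at once and then calls SaveSelf, which saves the object to the "LoginSaveGame" slot for user index 0.
; The password is held as a plain variable with no hashing or encryption shown.
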(fn RememberLoginInfo
  (return (Variables|Default|GetbRememberLoginInfo)))

(fn GetSavedUserName
  (return (Variables|Default|GetSavedUserName)))

(fn GetSavedPassword
  (return (Variables|Default|GetSavedPassword)))

(fn SaveSelf
  (SaveGame|SaveGametoSlot self "LoginSaveGame"))

(fn SetData
  (params (bRememberLoginInfo :type Boolean) (SavedUserName :type String) (SavedPassword :type String) (bAsGuest :type Boolean))
  (Variables|Default|SetbRememberLoginInfo bRememberLoginInfo)
  (Variables|Default|SetSavedUserName SavedUserName)
  (Variables|Default|SetSavedPassword SavedPassword)
  (Variables|Default|SetbAsGuest bAsGuest)
  (CallFunction|SaveSelf))

(fn IsGuest
  (return (Variables|Default|GetbAsGuest)))